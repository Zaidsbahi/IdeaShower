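; Sound manager Blueprint that controls fading of ambient audio for three locations: Yard, Cell and Cantine.
; Each location has an audio component with a pair of custom events that fade it in or out, using that location's fade length variable.
; BeginPlay triggers the Yard fade-out, and only the Yard events print debug text.
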(event Custom|Sound_Cantine_FadeOut
  ;[1 1 1] Cantine
  (Audio|Components|Audio|FadeOut (Variables|Default|GetCantine) (Variables|Default|GetCantineFadeLength) 0.0 "Linear" :!class /Script/Engine.AudioComponent))

(event Custom|Sound_Cantine_FadeIn
  ;[1 1 1] Cantine
  (Audio|Components|Audio|FadeIn (Variables|Default|GetCantine) (Variables|Default|GetCantineFadeLength) 1.0 0.0 "Linear" :!class /Script/Engine.AudioComponent))

(event Custom|Sound_Cell_FadeOut
  ;[1 1 1] Cell
  (Audio|Components|Audio|FadeOut (Variables|Default|GetCell) (Variables|Default|GetCellFadeLength) 0.0 "Linear" :!class /Script/Engine.AudioComponent))

(event Custom|Sound_Cell_FadeIn
  ;[1 1 1] Cell
  (Audio|Components|Audio|FadeIn (Variables|Default|GetCell) (Variables|Default|GetCellFadeLength) 1.0 0.0 "Linear" :!class /Script/Engine.AudioComponent))

(event Custom|Sound_Yard_FadeOut
  ;[1 1 1] Yard
  (Audio|Components|Audio|FadeOut (Variables|Default|GetYard) (Variables|Default|GetYardFadeLength) 0.0 "Linear" :!class /Script/Engine.AudioComponent)
  (Development|PrintText "yard amb. faded out"))

(event Custom|Sound_Yard_FadeIn
  ;[1 1 1] Yard
  (Audio|Components|Audio|FadeIn (Variables|Default|GetYard) (Variables|Default|GetYardFadeLength) 1.0 0.0 "Linear" :!class /Script/Engine.AudioComponent)
  (Development|PrintText "yard amb. faded in"))

(event EventBeginPlay
  (CallFunction|SoundYardFadeOut))

(event Collision|EventActorBeginOverlap
  (params (OtherActor :type Actor%20Object%20Reference)))

(event EventTick
  (params (DeltaSeconds :type Float%20%28single-precision%29)))

(fn ConstructionScript)