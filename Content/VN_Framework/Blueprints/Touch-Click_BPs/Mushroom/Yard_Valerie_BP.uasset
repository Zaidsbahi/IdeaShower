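; Yard_Valerie_BP is a touch-click actor in the visual novel that picks which Valerie yard scene to play.
; PickLocalScene walks nested MasterChoiceLog flags from the Global_BP game instance, returning a scene nickname for the worm, main or earlier diffuse and punch outcomes.
; Once the final flag is set, it hides the actor and disables input.
; The missing-scene debug print is disconnected, so unmatched states give no warning.
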(event EventBeginPlay
  (|CallParentFunction)
  (bind _asglobal_bp (Utilities|Casting|CastToGlobal_BP (Game|GetGameInstance)))
  (Variables|Default|SetAs%20Global%20BP _asglobal_bp))

(event Collision|EventActorBeginOverlap
  (params (OtherActor :type Actor%20Object%20Reference))
  (|CallParentFunction OtherActor) ; This node is disabled and will not be called.\nDrag off pins to build functionality.
)

(event EventTick
  (params (DeltaSeconds :type Float%20%28single-precision%29))
  (|CallParentFunction DeltaSeconds) ; This node is disabled and will not be called.\nDrag off pins to build functionality.
)

(fn ConstructionScript
  (|CallParentFunction))

(fn PickLocalScene
  (bind _asglobal_bp (Utilities|Casting|CastToGlobal_BP (Game|GetGameInstance)))
  (if (== (Utilities|Array|Get(acopy) (Variables|/Game/VN_Framework/Blueprints/Global_BP.Global_BP_C|GetMasterChoiceLog _asglobal_bp) 74) 0)
    (if (== (Utilities|Array|Get(acopy) (Variables|/Game/VN_Framework/Blueprints/Global_BP.Global_BP_C|GetMasterChoiceLog _asglobal_bp) 62) 1)
      (if (== (Utilities|Array|Get(acopy) (Variables|/Game/VN_Framework/Blueprints/Global_BP.Global_BP_C|GetMasterChoiceLog _asglobal_bp) 73) 1)
        (return "Yard_V_Main_Worm" false false)
        (elif (== (Utilities|Array|Get(acopy) (Variables|/Game/VN_Framework/Blueprints/Global_BP.Global_BP_C|GetMasterChoiceLog _asglobal_bp) 60) 1)
          (return "Yard_V_Main_Second" false false)
          (else
            (return "Yard_V_Main_First" false false))))
      (elif (== (Utilities|Array|Get(acopy) (Variables|/Game/VN_Framework/Blueprints/Global_BP.Global_BP_C|GetMasterChoiceLog _asglobal_bp) 51) 1)
        (return "Yard_V_Diffuse" false false)
        (elif (== (Utilities|Array|Get(acopy) (Variables|/Game/VN_Framework/Blueprints/Global_BP.Global_BP_C|GetMasterChoiceLog _asglobal_bp) 50) 1)
          (return "Yard_V_Punch" false false))))
    (else
      (CallFunction|HideActor)
      (Input|DisableInput 0))))