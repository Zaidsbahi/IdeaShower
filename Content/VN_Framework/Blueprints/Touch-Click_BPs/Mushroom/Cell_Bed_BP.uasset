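; Touch/click bed in the cell, part of the Mushroom set, that picks which visual novel scene to play.
; PickLocalScene reads an entry in the Global_BP game instance's MasterChoiceLog to choose the Cell_End scene or the default Cell_Bed scene, flagging when the ending is chosen.
; SceneEnd checks that flag and, if set, adds the EndScreens widget to the viewport.
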(event EventBeginPlay
  (|CallParentFunction) ; This node is disabled and will not be called.\nDrag off pins to build functionality.
)

(event Collision|EventActorBeginOverlap
  (params (OtherActor :type Actor%20Object%20Reference))
  (|CallParentFunction OtherActor) ; This node is disabled and will not be called.\nDrag off pins to build functionality.
)

(event EventTick
  (params (DeltaSeconds :type Float%20%28single-precision%29))
  (|CallParentFunction DeltaSeconds) ; This node is disabled and will not be called.\nDrag off pins to build functionality.
)

(fn ConstructionScript
  (|CallParentFunction))

(fn PickLocalScene
  (bind _asglobal_bp (Utilities|Casting|CastToGlobal_BP (Game|GetGameInstance)))
  (if (== (Utilities|Array|Get(acopy) (Variables|/Game/VN_Framework/Blueprints/Global_BP.Global_BP_C|GetMasterChoiceLog _asglobal_bp) 74) 1)
    (Variables|Default|SetEndSceneHasPlayed true)
    (return "Cell_End" false false)
    (else
      (return "Cell_Bed" false false))))

(fn SceneEnd
  (params (SceneTemplateBP :type Scene%20Template%20BP%20Object%20Reference) (next_scene :type String) (next_subLevel :type String) (next%20map%20Level :type String))
  (if (Variables|Default|GetEndSceneHasPlayed)
    (bind _returnvalue (UserInterface|CreateWidget "/Game/VN_Framework/ArtAssets/UI/Mushroom/End_Screens/EndScreens.EndScreens_C"))
    (UserInterface|Viewport|AddtoViewport _returnvalue 0)
    (Development|PrintText "end scene played")
    (else
      (Development|PrintText "end scene not yet played")))
  (return false))