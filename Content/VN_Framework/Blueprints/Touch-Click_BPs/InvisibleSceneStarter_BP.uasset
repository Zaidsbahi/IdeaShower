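; Invisible scene starter for the visual novel framework, with empty click, touch and interact handlers so player input does nothing.
; Its local scene pick returns the global current scene name, with travel prompt and breakdown skip both off.
; Helper graphs either show the credits widget after a delay, or build a spawned scene template and start its event with next level and sublevel.
; Side-scene and custom scene hooks are empty stubs.
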(event EventBeginPlay)

(event Collision|EventActorBeginOverlap
  (params (OtherActor :type Actor%20Object%20Reference)))

(event EventInteract)

(event EventActorOnInputTouchBegin
  (params (FingerIndex :type ETouchIndex%20Enum :default "Touch1"))
  ;[1 0.00954 0.04934] Do nothing if clicked
)

(event EventTick
  (params (DeltaSeconds :type Float%20%28single-precision%29)))

(event MouseInput|EventActorOnClicked
  (params (ButtonPressed :type Key%20Structure :default "None"))
  ;[1 0.00954 0.04934] Do nothing if clicked
)

(fn ConstructionScript
  (|CallParentFunction))

(fn CheckSideScenes)

(fn ScenesPart3
  (if false
    _))

(fn PickLocalScene
  (return (Variables|/Game/VN_Framework/Blueprints/Global_BP.Global_BP_C|GetcurrentScene (Variables|Default|GetGlobal_BP)) false false))

(fn CustomSceneCode
  (return))