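; Follow spotlight that tracks the player and swings to highlight objects they interact with or approach.
; It starts hidden, then fades in by timeline after a long BeginPlay delay, guarded to run once.
; Each Tick scans for overlapped TouchClickActor_BP actors during interaction, otherwise for near or moving tagged inspectables, easing rotation and switching intensity.
; It returns to the player for Ignore-tagged actors, or without an active inspectable unless the character's LightTracking is set.
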(event Custom|StartingLightsAfterSceneEnd
  (if (Variables|Default|GetCanSkip?)
    (bind _followlighttime (Timeline|FollowLightsTime Play)
      (:Update
        (Rendering|Components|Light|SetIntensity (Variables|Default|GetSpotLightComponent) (Math|Float|Lerp 0.0 (Variables|Default|GetLightOnPlayerIntensity) _followlighttime))
        (Variables|Default|SetCanSkip? false)
        (Rendering|SetActorHiddenInGame false)))))

(event EventTick
  (params (DeltaSeconds :type Float%20%28single-precision%29))
  (if (Variables|/Game/VN_Framework/Blueprints/Global_BP.Global_BP_C|GetIsInteractingWithObject? (Variables|Default|GetAs%20Global%20BP))
    (bind _outactors (Actor|GetAllActorsOfClass "/Game/VN_Framework/Blueprints/Touch-Click_BPs/TouchClickActor_BP.TouchClickActor_BP_C"))
    (for (_array_element _array_index) _outactors
      (if (Collision|IsOverlappingActor _array_element (Game|GetPlayerCharacter 0) :!class /Script/Engine.Actor)
        (if (not (Actor|ActorHasTag _array_element "Ignore"))
          (Transformation|SetWorldRotation (Variables|Default|GetSpotLightComponent) (Math|Interpolation|RInterpTo (.OutRotation (Actor|GetActorEyesViewPoint)) (Math|Rotator|FindLookatRotation (Transformation|GetActorLocation) (Transformation|GetActorLocation (Utilities|Array|Get(acopy) _outactors _array_index))) DeltaSeconds 5.0) false false)
          (Rendering|Components|Light|SetIntensity (Variables|Default|GetSpotLightComponent) (Variables|Default|GetLightOnOtherStuffIntensity))
          (else
            (CallFunction|RotateLighttoCharacter DeltaSeconds)))))
    (else
      (bind _outactors_2 (Actor|GetAllActorsOfClasswithTag "/Game/Zaid/Inspectables/ParentInspectables.ParentInspectables_C" "Inspectables"))
      (for (_array_element_2 _array_index_2) _outactors_2
        (if (or (Variables|/Game/Zaid/Inspectables/ParentInspectables.ParentInspectables_C|GetIsCharacterNear? _array_element_2) (Variables|/Game/Zaid/Inspectables/ParentInspectables.ParentInspectables_C|GetIsMoving _array_element_2))
          (bind _output_get (Variables|Default|SetCurrentActorPlace (Utilities|Array|Get(acopy) _outactors_2 _array_index_2))))
        (Utilities|IsValid _output_get
          (:Is%20Valid
            (if (or (Variables|/Game/Zaid/Inspectables/ParentInspectables.ParentInspectables_C|GetIsCharacterNear? _output_get) (Variables|/Game/Zaid/Inspectables/ParentInspectables.ParentInspectables_C|GetIsMoving _output_get))
              (Transformation|SetWorldRotation (Variables|Default|GetSpotLightComponent) (Math|Interpolation|RInterpTo (.OutRotation (Actor|GetActorEyesViewPoint)) (Math|Rotator|FindLookatRotation (Transformation|GetActorLocation) (Transformation|GetActorLocation (Variables|Default|GetCurrentActorPlace))) DeltaSeconds 5.0) false false)
              (Rendering|Components|Light|SetIntensity (Variables|Default|GetSpotLightComponent) (Variables|Default|GetLightOnOtherStuffIntensity))
              (else
                (if (not (Variables|/Game/VN_Framework/Blueprints/VN_FirstPersonCharacter.VN_FirstPersonCharacter_C|GetLightTracking (Variables|Default|GetAs%20VN%20First%20Person%20Character))) :!label _label
                  (CallFunction|RotateLighttoCharacter DeltaSeconds)))))
          (:Is%20Not%20Valid
            (goto _label)))))))

(event EventBeginPlay
  (bind _asvn_first_person_character (Utilities|Casting|CastToVN_FirstPersonCharacter (Game|GetPlayerCharacter 0)))
  (Variables|Default|SetAs%20VN%20First%20Person%20Character _asvn_first_person_character)
  (Variables|Default|SetCanSkip? true)
  (Variables|Default|SetIsOverlappingShard? false)
  (bind _asglobal_bp (Utilities|Casting|CastToGlobal_BP (Game|GetGameInstance)))
  (Variables|Default|SetAs%20Global%20BP _asglobal_bp)
  (Rendering|SetActorHiddenInGame true)
  (Utilities|FlowControl|Delay 108.0)
  (CallFunction|StartingLightsAfterSceneEnd)
  (Rendering|SetActorHiddenInGame false))

(fn ConstructionScript)

(fn RotateLighttoCharacter
  (params (DeltaSeconds :type Float%20%28double-precision%29))
  (Utilities|IsValid (Game|GetPlayerCharacter 0)
    (:Is%20Valid
      (Transformation|SetWorldRotation (Variables|Default|GetSpotLightComponent) (Math|Interpolation|RInterpTo (.OutRotation (Actor|GetActorEyesViewPoint)) (Math|Rotator|FindLookatRotation (Transformation|GetActorLocation) (Transformation|GetActorLocation (Game|GetPlayerCharacter 0))) DeltaSeconds 5.0) false false)
      (Rendering|Components|Light|SetIntensity (Variables|Default|GetSpotLightComponent) (Variables|Default|GetLightOnPlayerIntensity)))))

(fn RotateLighttoObject
  (bind _outactors (Actor|GetAllActorsOfClass "/Game/VN_Framework/Blueprints/Touch-Click_BPs/TouchClickActor_BP.TouchClickActor_BP_C"))
  (for (_array_element _array_index) _outactors
    (if (Collision|IsOverlappingActor _array_element (Game|GetPlayerCharacter 0) :!class /Script/Engine.Actor)
      (Transformation|SetWorldRotation (Variables|Default|GetSpotLightComponent) (Math|Rotator|FindLookatRotation (Transformation|GetActorLocation) (Transformation|GetActorLocation (Utilities|Array|Get(acopy) _outactors _array_index))) false false))))