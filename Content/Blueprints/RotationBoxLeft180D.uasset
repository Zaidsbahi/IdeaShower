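; Trigger box that rotates platforms left or right when the player character overlaps it.
; The direction comes from its RotateRight flag and is gated by the RotatedLeft or RotatedRight state of the first RotationPivot, cached at BeginPlay.
; It messages every BPUI_Rotate implementer, flips RotateRight and copies the new value to all RotatedFromDoor actors.
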(event OnComponentBeginOverlap(Box)
  (params (OverlappedComponent :type Primitive%20Component%20Object%20Reference) (OtherActor :type Actor%20Object%20Reference) (OtherComp :type Primitive%20Component%20Object%20Reference) (OtherBodyIndex :type Integer) (bFromSweep :type Boolean) (SweepResult :type Hit%20Result%20Structure%20%28by%20ref%29))
  (if (Math|Boolean|ANDBoolean (== OtherActor (Game|GetPlayerCharacter 0)) (Variables|Default|GetRotateRight?) (Variables|/Game/Blueprints/RotationPivot.RotationPivot_C|GetRotatedLeft? (Utilities|Array|Get(acopy) (stale EventBeginPlay _outactors))))
    (bind _outactors (Actor|GetAllActorswithInterface "/Game/Blueprints/Interfaces/BPUI_Rotate.BPUI_Rotate_C"))
    (for _array_element _outactors
      (Class|BPUIRotate|RotatePlatformRight(Message) _array_element)
      (Variables|Default|SetRotateRight? false)
      (bind _outactors_2 (Actor|GetAllActorsOfClass "/Game/Blueprints/RotatedFromDoor.RotatedFromDoor_C"))
      (for _array_element_2 _outactors_2
        (Variables|/Game/Blueprints/RotatedFromDoor.RotatedFromDoor_C|SetRotateRight? _array_element_2 true)))
    (elif (Math|Boolean|ANDBoolean (== OtherActor (Game|GetPlayerCharacter 0)) (not (Variables|Default|GetRotateRight?)) (Variables|/Game/Blueprints/RotationPivot.RotationPivot_C|GetRotatedRight? (Utilities|Array|Get(acopy) (stale EventBeginPlay _outactors))))
      (bind _outactors_3 (Actor|GetAllActorswithInterface "/Game/Blueprints/Interfaces/BPUI_Rotate.BPUI_Rotate_C"))
      (for _array_element_3 _outactors_3
        (Class|BPUIRotate|RotatePlatformLeft(Message) _array_element_3)
        (Variables|Default|SetRotateRight? true)
        (bind _outactors_4 (Actor|GetAllActorsOfClass "/Game/Blueprints/RotatedFromDoor.RotatedFromDoor_C"))
        (for _array_element_4 _outactors_4
          (Variables|/Game/Blueprints/RotatedFromDoor.RotatedFromDoor_C|SetRotateRight? _array_element_4 false))))))

(event EventBeginPlay
  (bind _outactors (Actor|GetAllActorsOfClass "/Game/Blueprints/RotationPivot.RotationPivot_C")))

(fn ConstructionScript)