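; Rotation pivot actor, apparently for stairs, that turns and shifts vertically as the player nears a proximity marker.
; Each Tick maps player distance to the first StairsProximity actor, found at BeginPlay, onto a clamped alpha that lerps yaw and Z toward MaxRotation and MaxDescent.
; Separate events turn the root 90 degrees left or right through timelines.
; StairsSmoothRotation only stores rotation targets, and several earlier experiments remain disconnected.
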(event EventRotatePlatformRight
  (bind _returnvalue (Transformation|GetActorRotation))
  (Development|PrintString "Rotate Right")
  (Variables|Default|SetActorInitialRotation (Transformation|GetActorRotation))
  (Variables|Default|SetActorTargetLocation (Math|Rotator|MakeRotator (.roll _returnvalue) (.pitch _returnvalue) (+ (.yaw _returnvalue) 9e+01)))
  (bind _rotationspeed (Timeline|Rotation PlayFromStart)
    (:Update
      (Transformation|SetWorldRotation (Variables|Default|GetDefaultSceneRoot) (Math|Rotator|Lerp(Rotator) (Variables|Default|GetActorInitialRotation) (Variables|Default|GetActorTargetLocation) _rotationspeed) false false))))

(event EventRotatePlatformLeft
  (bind _returnvalue (Transformation|GetActorRotation))
  (Development|PrintString "Rotate Left")
  (Variables|Default|SetActorInitialRotation (Transformation|GetActorRotation))
  (Variables|Default|SetActorTargetLocation (Math|Rotator|MakeRotator (.roll _returnvalue) (.pitch _returnvalue) (+ (.yaw _returnvalue) -9e+01)))
  (bind _rotationspeed (Timeline|Timeline PlayFromStart)
    (:Update
      (Transformation|SetWorldRotation (Variables|Default|GetDefaultSceneRoot) (Math|Rotator|Lerp(Rotator) (Variables|Default|GetActorInitialRotation) (Variables|Default|GetActorTargetLocation) _rotationspeed) false false))))

(event EventTick
  (params (DeltaSeconds :type Float%20%28single-precision%29))
  (bind _returnvalue (Game|GetPlayerCharacter 0))
  (bind _target_point (Variables|Default|GetTarget%20Point))
  (bind _triggerdistance_ (Variables|Default|GetTriggerDistance%20))
  (bind _returnvalue_2 (Transformation|GetActorLocation _target_point))
  (bind _returnvalue_3 (Transformation|GetActorLocation _returnvalue))
  (bind _returnvalue_4 (Math|Vector|Distance(Vector) _returnvalue_2 _returnvalue_3))
  (bind _returnvalue_5 (/ _returnvalue_4 _triggerdistance_))
  (bind _returnvalue_6 (- 1.0 _returnvalue_5))
  (bind _returnvalue_7 (Math|Float|Clamp(Float) _returnvalue_6))
  (Utilities|IsValid _returnvalue
    (:Is%20Valid
      (Development|PrintString (Utilities|String|ToString(Float) _returnvalue_4))
      (Transformation|SetActorRotation (Math|Rotator|MakeRotator 0.0 0.0 (Math|Float|Lerp 0.0 (Variables|Default|GetMaxRotation) _returnvalue_7)))
      (Transformation|SetActorLocation (Math|Vector|MakeVector 0.0 0.0 (Math|Float|Lerp (.z (Variables|Default|GetStairsInitialTransform)) (Variables|Default|GetMaxDescent%20) _returnvalue_7)) false false))))

(event EventStairsSmoothRotation
  (bind _returnvalue (Transformation|GetActorRotation))
  (Development|PrintString "SmoothStairs")
  (Variables|Default|SetActorInitialRotation (Transformation|GetActorRotation))
  (Variables|Default|SetActorTargetLocation (Math|Rotator|MakeRotator (.roll _returnvalue) (.pitch _returnvalue) (+ (.yaw _returnvalue) 9e+01))))

(event EventBeginPlay
  (Variables|Default|SetStairsInitialTransform (Transformation|GetActorLocation))
  (Variables|Default|SetStairsRotationInitial (Transformation|GetActorRotation))
  (Variables|Default|SetStairsRotationLocation (Math|Rotator|MakeRotator (.roll (Variables|Default|GetStairsRotationInitial)) (.pitch (Variables|Default|GetStairsRotationInitial)) (+ (.yaw (Variables|Default|GetStairsRotationInitial)) 2e+02)))
  (bind _outactors (Actor|GetAllActorsOfClass "/Game/Zaid/StairStageRotate/StairsProximity.StairsProximity_C"))
  (Variables|Default|SetTarget%20Point (Utilities|Array|Get(acopy) _outactors)))

(fn ConstructionScript)

(fn RotateWorld
  (Development|PrintString "Rotate")
  (Transformation|SetWorldRotation (Variables|Default|GetDefaultSceneRoot) "90.000000,90.000000,90.000000" false false))